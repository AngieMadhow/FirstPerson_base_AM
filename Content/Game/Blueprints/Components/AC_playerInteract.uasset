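; Player interaction component that finds interactable actors in the first-person camera's line of sight.
; On BeginPlay it casts its owner to BP_FirstPersonCharacter and caches that reference.
; Its LineTrace function traces the Visibility channel forward from the camera over a given length, with debug drawing left on.
; It returns the hit actor only if it implements BPI_Interactable; the interaction call itself is not made here.
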(event EventBeginPlay
  ;[0.15 0.15 0.15 0.5] recuperer le joueur
  (bind _asbp_first_person_character (Utilities|Casting|CastToBP_FirstPersonCharacter (Components|GetOwner)))
  (Variables|Default|SetplayerRef _asbp_first_person_character))

(event EventTick
  (params (DeltaSeconds :type Float%20%28single-precision%29)))

(fn LineTrace
  (params (Lenght :type Float%20%28double-precision%29))
  (bind _playerref (Variables|Default|GetplayerRef))
  (bind _firstpersoncamera (Variables|/Game/Game/Blueprints/Pawns_Characters/Player/FirstPerson/Blueprints/BP_FirstPersonCharacter.BP_FirstPersonCharacter_C|GetFirstPersonCamera _playerref))
  (bind _returnvalue (Transformation|GetWorldLocation _firstpersoncamera))
  ;[0.15 0.15 0.15 0.5] tracer la ligne
  (bind _outhit (Collision|LineTraceByChannel _returnvalue (+ _returnvalue (* (Math|Vector|GetForwardVector _firstpersoncamera) Lenght)) "TraceTypeQuery1" false 0 "ForDuration"))
  (if (and (Utilities|IsValid (.HitActor (Collision|BreakHitResult _outhit))) (Utilities|DoesObjectImplementInterface (.HitActor (Collision|BreakHitResult _outhit)) "/Game/Game/Blueprints/Interfaces/BPI_Interactable.BPI_Interactable_C"))
    (return (.HitActor (Collision|BreakHitResult _outhit)))
    (else
      (return 0))))