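; BP_lightOn is an interactable light switch actor that toggles a referenced light.
; On Interact, a FlipFlop tilts the Interrupteur component between two opposite angles.
; The same event inverts the visibility of the assigned Light if valid, independently of the switch's FlipFlop state.
; Turning the light off also applies MI_FirstPersonColorway through SetMaterial, with no material change when turning it on.
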(event EventBeginPlay)

(event Collision|EventActorBeginOverlap
  (params (OtherActor :type Actor%20Object%20Reference)))

(event EventTick
  (params (DeltaSeconds :type Float%20%28single-precision%29)))

(event EventInteract
  (params (Actor :type Actor%20Object%20Reference))
  (bind _interrupteur (Variables|Default|Getinterrupteur))
  (bind _light (Variables|Default|Getlight))
  (bind _lightcomponent (Variables|/Script/Engine.Light|GetLightComponent _light))
  (Utilities|FlowControl|Sequence
    (:then_0
      ;[0.15 0.15 0.15 0.5] filp interrupteur
      (Utilities|FlowControl|FlipFlop
        (:A
          (Transformation|SetRelativeRotation _interrupteur "-10.000000,0.000000,0.000000" false false))
        (:B
          (Transformation|SetRelativeRotation _interrupteur "10.000000,0.000000,0.000000" false false))))
    (:then_1
      (Utilities|IsValid _light
        (:Is%20Valid
          (if (Variables|/Script/Engine.SceneComponent|GetbVisible _lightcomponent)
            (Rendering|SetVisibility _lightcomponent false false)
            (Rendering|Material|SetMaterial 0 "/Game/Game/Blueprints/Pawns_Characters/Player/FirstPerson/MI_FirstPersonColorway.MI_FirstPersonColorway")
            (else
              (Rendering|SetVisibility _lightcomponent true false))))))))

(fn ConstructionScript)